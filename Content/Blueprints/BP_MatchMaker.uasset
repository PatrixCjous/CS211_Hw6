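; BP_MatchMaker is a Blueprint that automatically hosts or joins a LAN multiplayer session when play begins.
; On BeginPlay it searches for LAN sessions with the first player controller and joins the first result.
; If none are found, it creates a small LAN session and opens the level named by LevelString as a listen server.
; Only success paths are wired, so failed searches, creations and joins go unhandled.
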(event `self.ReceiveBeginPlay`
  (bind _results (`FindSessionsCallbackProxy.FindSessions` (`GameplayStatics.GetPlayerController` 0) 4 true)
    (:`OnSuccess`
      (if (== (`KismetArrayLibrary.Array_Length` _results) 0)
        (`CreateSessionCallbackProxy.CreateSession` (`GameplayStatics.GetPlayerController` 0) 4 true
          (:`OnSuccess`
            (`GameplayStatics.OpenLevel` (`self.LevelString`) true "listen")))
        (else
          (`JoinSessionCallbackProxy.JoinSession` (`GameplayStatics.GetPlayerController` 0) (`KismetArrayLibrary.Array_Get` _results)))))))

(fn `UserConstructionScript`)