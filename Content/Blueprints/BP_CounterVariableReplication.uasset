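; Replication demo actor that displays a running counter on a text component.
; On BeginPlay, only the authority starts a looping timer that calls UpdateCount to increment Count every couple of seconds.
; Tick runs without an authority check and writes the current Count to CounterText each frame.
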(event `self.ReceiveBeginPlay`
  (`/Engine/EditorBlueprintResources/ActorMacros.Switch Has Authority`
    (:`Authority`
      (`KismetSystemLibrary.K2_SetTimer` null "UpdateCount" 2.0 true))))

(event `self.ReceiveTick`
  (params (DeltaSeconds :type "Float (single-precision)"))
  (`TextRenderComponent.SetText` (`self.CounterText`) (`KismetStringLibrary.Conv_IntToString` (`self.Count`))))

(fn `UpdateCount`
  (set `self.Count` (+ (`self.Count`) 1)))

(fn `UserConstructionScript`)