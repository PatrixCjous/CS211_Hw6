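; Replication example actor that demonstrates a RepNotify variable through a visible counter.
; On BeginPlay, only the authority starts a looping timer that calls UpdateCount every couple of seconds to increment Count.
; The OnRep_Count notify reacts to each change by spawning an explosion emitter at the CounterText location and updating that text to the new value.
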(event `self.ReceiveBeginPlay`
  (`/Engine/EditorBlueprintResources/ActorMacros.Switch Has Authority`
    (:`Authority`
      (`KismetSystemLibrary.K2_SetTimer` null "UpdateCount" 2.0 true))))

(fn `OnRep_Count`
  (`GameplayStatics.SpawnEmitterAtLocation` "/Game/StarterContent/Particles/P_Explosion.P_Explosion" (`SceneComponent.K2_GetComponentLocation` (`self.CounterText`)))
  (`TextRenderComponent.SetText` (`self.CounterText`) (`KismetStringLibrary.Conv_IntToString` (`self.Count`))))

(fn `UpdateCount`
  (set `self.Count` (+ (`self.Count`) 1)))

(fn `UserConstructionScript`)