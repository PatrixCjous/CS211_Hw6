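; BP_LegoBlock is an interactable object that can switch among furniture, electronics, plant and civil-engineering meshes, and is destroyed on the server when interacted with.
; ChangePreview multicasts from the server or applies locally on clients.
; ChangeShape replaces all mesh components using wrapped category and item indices, flagging the civil-engineering category as Workbenchable.
; A Disappear timeline can fade material opacity, with dynamic instances created at BeginPlay.
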(event `self.ReceiveBeginPlay`
  (for _array_element (`self.K2_GetComponentsByClass` "/Script/Engine.StaticMeshComponent")
    (bind _returnvalue (`PrimitiveComponent.CreateDynamicMaterialInstance` _array_element 0 "/Game/Homework/Materials/M_LegoBlock.M_LegoBlock"))
    (set `self.blockMat` _returnvalue)))

(event `self.Interact`
  (for _ (`self.K2_GetComponentsByClass` "/Script/Engine.StaticMeshComponent")
    (`/Engine/EditorBlueprintResources/ActorMacros.Switch Has Authority`
      (:`Authority`
        (`self.K2_DestroyActor`)))))

(event `Disappear`
  (bind (_direction _opacity) (`Timeline|fadeAnim` :!via `PlayFromStart`)
    (:`Update`
      (for _array_element (`self.K2_GetComponentsByClass` "/Script/Engine.StaticMeshComponent")
        (for _array_element_2 (`MeshComponent.GetMaterials` _array_element)
          (bind _asmaterial_instance_dynamic (cast `MaterialInstanceDynamic` _array_element_2))
          (`MaterialInstanceDynamic.SetScalarParameterValue` _asmaterial_instance_dynamic "Opa" _opacity))))))

(event `self.Change_Preview`
  (params (ClassIndex :type Integer) (ObjectIndex :type Integer))
  (`/Engine/EditorBlueprintResources/ActorMacros.Switch Has Authority`
    (:`Authority`
      (`self.Multicast Change Shape` ClassIndex ObjectIndex))
    (:`Remote`
      (`self.changeShape` ClassIndex ObjectIndex))))

(event `Multicast Change Shape`
  (params (ClassNum :type Integer :default 0) (ObjNum :type Integer :default 0))
  (`self.changeShape` ClassNum ObjNum))

(fn `changeShape`
  (params (ClassNum :type Integer) (ObjNum :type Integer))
  (bind _chairs (`self.Chairs`))
  (bind _tables (`self.Tables`))
  (bind _computers (`self.Computers`))
  (bind _tvs (`self.TVs`))
  (bind _plants (`self.Plants`))
  (bind _civilengineeringtoolkit (`self.CivilEngineeringToolkit`))
  (bind _returnvalue (mod ClassNum (`self.NumClasses`)))
  (set `self.OldClassNum` ClassNum)
  (set `self.OldObjNum` ObjNum)
  (switch `int` _returnvalue
    (:`0`
      (set `self.StaticMesh` (`KismetArrayLibrary.Array_Get` _chairs (mod ObjNum (`KismetArrayLibrary.Array_Length` _chairs)))))
    (:`1`
      (set `self.StaticMesh` (`KismetArrayLibrary.Array_Get` _tables (mod ObjNum (`KismetArrayLibrary.Array_Length` _tables)))))
    (:`2`
      (set `self.StaticMesh` (`KismetArrayLibrary.Array_Get` _tvs (mod ObjNum (`KismetArrayLibrary.Array_Length` _tvs)))))
    (:`3`
      (set `self.StaticMesh` (`KismetArrayLibrary.Array_Get` _computers (mod ObjNum (`KismetArrayLibrary.Array_Length` _computers)))))
    (:`4`
      (set `self.StaticMesh` (`KismetArrayLibrary.Array_Get` _plants (mod ObjNum (`KismetArrayLibrary.Array_Length` _plants)))))
    (:`5`
      (set `self.StaticMesh` (`KismetArrayLibrary.Array_Get` _civilengineeringtoolkit (mod (`KismetArrayLibrary.Array_Length` _civilengineeringtoolkit) ObjNum)))))
  (for _array_element (`self.K2_GetComponentsByClass` "/Script/Engine.StaticMeshComponent")
    (`ActorComponent.K2_DestroyComponent` _array_element))
  (bind _returnvalue_2 (`AddComponent|Static Mesh Component_22332`))
  (`StaticMeshComponent.SetStaticMesh` _returnvalue_2 (`self.StaticMesh`))
  (set `self.Workbenchable` (== 5 _returnvalue)))

(fn `UserConstructionScript`
  (bind _chairs (`self.Chairs`))
  (bind _tvs (`self.TVs`))
  (bind _computers (`self.Computers`))
  (bind _plants (`self.Plants`))
  (`|ExecutionSequence`
    (:`then_0`
      (set `self.NumClasses` 6))
    (:`then_1`
      (`KismetArrayLibrary.Array_Add` _chairs "/Game/Homework/Meshes/RollingChair.RollingChair")
      (`KismetArrayLibrary.Array_Add` _chairs "/Game/Homework/Meshes/SmallChair.SmallChair")
      (`KismetArrayLibrary.Array_Add` _chairs "/Game/Homework/Meshes/SmallChair2.SmallChair2"))
    (:`then_2`
      (`KismetArrayLibrary.Array_Add` (`self.Tables`) "/Game/StarterContent/Props/SM_TableRound.SM_TableRound"))
    (:`then_3`
      (`KismetArrayLibrary.Array_Add` _tvs "/Game/Homework/Meshes/FlatScreenTV.FlatScreenTV")
      (`KismetArrayLibrary.Array_Add` _tvs "/Game/Homework/Meshes/CRT.CRT"))
    (:`then_4`
      (`KismetArrayLibrary.Array_Add` _computers "/Game/Homework/Meshes/Laptop.Laptop")
      (`KismetArrayLibrary.Array_Add` _computers "/Game/Homework/Meshes/Clock.Clock"))
    (:`then_5`
      (`KismetArrayLibrary.Array_Add` _plants "/Game/Homework/Meshes/Flower.Flower")
      (`KismetArrayLibrary.Array_Add` _plants "/Game/StarterContent/Props/SM_Bush.SM_Bush")
      (`KismetArrayLibrary.Array_Add` _plants "/Game/Homework/Meshes/Cactus.Cactus"))
    (:`then_6`
      (`KismetArrayLibrary.Array_Add` (`self.CivilEngineeringToolkit`) "/Game/Homework/Blueprints/Workbench/SmallBuilding.SmallBuilding"))))