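; Room button actor that loads the level named in its Level variable when it receives a trace-hit event.
; The event prints a debug string, then calls Open Level.
; A disconnected, never-run chain would offset the button by ChangeX and ChangeY, send ChangeRoomsMessage to each wall in WallsToClose, and give every BP_RoomJoin the new spawn location while marking it ready to join.
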(event `self.TraceHitActorWithComponent`
  (params (Component :type "PrimitiveComponent Object Reference") (Actor :type "Actor Object Reference"))
  (`KismetSystemLibrary.PrintString` "Algo")
  (`GameplayStatics.OpenLevel` (`self.Level`)))

(fn `UserConstructionScript`)