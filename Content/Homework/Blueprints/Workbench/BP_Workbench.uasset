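; BP_Workbench turns a miniature LEGO layout into constructed buildings in a networked VR game.
; GetBuildings gathers overlapping workbenchable BP_LegoBlocks and stores each one's rotation and offset from the Box.
; ConstructBuilding spawns BP_ConstructSmallBuildings for blocks using the SmallBuilding mesh, at ten times those offsets from the world origin.
; It then relocates every NetworkedVRChar to a fixed position through RelocatePlayerServer.
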(event `self.ReceiveBeginPlay`)

(event `self.ReceiveTick`
  (params (DeltaSeconds :type "Float (single-precision)")))

(event `self.getBuildings`
  (params (Character :type "/Game/Blueprints/NetworkedVRChar Object Reference"))
  (for _array_element (`PrimitiveComponent.GetOverlappingActors` "/Game/Homework/Blueprints/BP_LegoBlock.BP_LegoBlock_C")
    (bind _asbp_lego_block (cast `/Game/Homework/Blueprints/BP_LegoBlock` _array_element))
    (if (`/Game/Homework/Blueprints/BP_LegoBlock.Workbenchable` _asbp_lego_block)
      (`KismetArrayLibrary.Array_Add` (`self.Locations`) (`KismetMathLibrary.MakeTransform` (- (`self.K2_GetActorLocation` _array_element) (`SceneComponent.K2_GetComponentLocation` (`self.Box`))) (`self.K2_GetActorRotation` _array_element)))
      (`KismetArrayLibrary.Array_Add` (`self.Buildings`) _array_element)))
  (`self.Construct Building` (`self.Buildings`)))

(event `Construct Building`
  (params (Buildings :type "Array of Actor Object Reference"))
  (for (_array_element _array_index) Buildings
    (bind _asbp_lego_block (cast `/Game/Homework/Blueprints/BP_LegoBlock` _array_element))
    (if (== "/Game/Homework/Blueprints/Workbench/SmallBuilding.SmallBuilding" (`/Game/Homework/Blueprints/BP_LegoBlock.StaticMesh` _asbp_lego_block))
      (`|SpawnActorFromClass` "/Game/Homework/Blueprints/Workbench/BP_ConstructSmallBuildings.BP_ConstructSmallBuildings_C" (`KismetMathLibrary.MakeTransform` (+ (* (.location (`KismetArrayLibrary.Array_Get` (`self.Locations`) _array_index)) 10.0) (0.0 0.0 0.0)) (.rotation (`KismetArrayLibrary.Array_Get` (`self.Locations`) _array_index)) (.scale (`KismetArrayLibrary.Array_Get` (`self.Locations`) _array_index))))
      (`KismetArrayLibrary.Array_Add` (`self.NewBuildings`))))
  (bind _outactors (`GameplayStatics.GetAllActorsOfClass` "/Game/Blueprints/NetworkedVRChar.NetworkedVRChar_C"))
  (for _array_element_2 _outactors
    (`/Game/Blueprints/NetworkedVRChar.RelocatePlayerServer` _array_element_2 (470.0 470.0 540.0))))

(fn `UserConstructionScript`)