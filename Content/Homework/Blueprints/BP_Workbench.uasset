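; BP_Workbench is a workbench actor that hands the Lego blocks placed on it to a VR character to start a simulation.
; When a NetworkedVRChar begins overlapping it, it sends a GetBuildings message and prints a debug string.
; GetBuildings gathers overlapping workbenchable BP_LegoBlocks and their offsets from the bench, then passes both arrays to the character's StartSimulation.
; Both arrays are appended to without being cleared here.
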(event `self.ReceiveBeginPlay`)

(event `self.ReceiveTick`
  (params (DeltaSeconds :type "Float (single-precision)")))

(event `self.getBuildings`
  (params (Character :type "/Game/Blueprints/NetworkedVRChar Object Reference"))
  (for _array_element (`PrimitiveComponent.GetOverlappingActors` "/Game/Homework/Blueprints/BP_LegoBlock.BP_LegoBlock_C")
    (bind _asbp_lego_block (cast `/Game/Homework/Blueprints/BP_LegoBlock` _array_element))
    (if (`/Game/Homework/Blueprints/BP_LegoBlock.Workbenchable` _asbp_lego_block)
      (`KismetArrayLibrary.Array_Add` (`self.Locations`) (- (`self.K2_GetActorLocation` _array_element) (`self.K2_GetActorLocation`)))
      (`KismetArrayLibrary.Array_Add` (`self.Buildings`) _array_element)))
  (`/Game/Blueprints/NetworkedVRChar.startSimulation` Character (`self.Buildings`) (`self.Locations`)))

(event `self.ReceiveActorBeginOverlap`
  (params (OtherActor :type "Actor Object Reference"))
  (bind _asnetworked_vrchar (cast `/Game/Blueprints/NetworkedVRChar` OtherActor))
  (message `/Game/Homework/Blueprints/BPI_EngineeringDemo.getBuildings` self _asnetworked_vrchar)
  (`KismetSystemLibrary.PrintString` "Hello"))

(fn `UserConstructionScript`)