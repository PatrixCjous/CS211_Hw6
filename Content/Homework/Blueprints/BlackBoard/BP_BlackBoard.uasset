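; BP_BlackBoard is a blackboard actor built at BeginPlay as a grid of spawned BP_Pixel actors, oriented to the actor's rotation.
; The construction script derives rows and columns from board size and scaled pixel size, creates a four-color dynamic material palette and sizes GridArray to match.
; Each pixel receives its grid index and a reference to the board, whose PixelUpdate event writes cell values into GridArray.
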(event `self.ReceiveBeginPlay`
  (`/Game/Homework/Blueprints/BlackBoard/BPC_GridArray.InitArray` (`self.GridArray`))
  (`self.BuildBlackBoard`))

(event `PixelUpdate`
  (params (i :type Integer :default 0) (j :type Integer :default 0) (value :type Integer :default 0))
  (`/Game/Homework/Blueprints/BlackBoard/BPC_GridArray.SetCell` (`self.GridArray`) i j value))

(fn `BuildBlackBoard`
  (bind _currentpixel (`self.currentPixel`))
  (for _index (range (`self.rows`))
    (for _index_2 (range (`self.columns`))
      (`|ExecutionSequence`
        (:`then_0`
          (bind _returnvalue (`|SpawnActorFromClass` "/Game/Homework/Blueprints/BlackBoard/BP_Pixel.BP_Pixel_C" (`KismetMathLibrary.MakeTransform` (`self.CellPosition` _index _index_2) (`self.K2_GetActorRotation`) (`self.PixelScaleVector`))))
          (set `self.currentPixel` _returnvalue))
        (:`then_1`
          (`/Game/Homework/Blueprints/BlackBoard/BP_Pixel.SetIndex` _currentpixel _index _index_2)
          (`/Game/Homework/Blueprints/BlackBoard/BP_Pixel.SetParent` _currentpixel self)
          (`KismetArrayLibrary.Array_Add` (`self.pixels`) _currentpixel))))))

(fn `BuildMaterialCollection`
  (bind _materialcollection (`self.materialCollection`))
  (bind _materialcollection_2 (`self.materialCollection`))
  (bind _materialcollection_3 (`self.materialCollection`))
  (bind _materialcollection_4 (`self.materialCollection`))
  (`|ExecutionSequence`
    (:`then_0`
      (bind _returnvalue (`KismetMaterialLibrary.CreateDynamicMaterialInstance` "/Game/Homework/Blueprints/BlackBoard/M_Pixel.M_Pixel"))
      (`KismetArrayLibrary.Array_Add` _materialcollection_2 _returnvalue)
      (`MaterialInstanceDynamic.SetVectorParameterValue` (`KismetArrayLibrary.Array_Get` _materialcollection_2) "Color" (`KismetMathLibrary.MakeColor` 1.0 1.0 1.0)))
    (:`then_1`
      (bind _returnvalue_2 (`KismetMaterialLibrary.CreateDynamicMaterialInstance` "/Game/Homework/Blueprints/BlackBoard/M_Pixel.M_Pixel"))
      (`KismetArrayLibrary.Array_Add` _materialcollection_3 _returnvalue_2)
      (`MaterialInstanceDynamic.SetVectorParameterValue` (`KismetArrayLibrary.Array_Get` _materialcollection_3 1) "Color" (`KismetMathLibrary.MakeColor` 1.0 0.0 0.0)))
    (:`then_2`
      (bind _returnvalue_3 (`KismetMaterialLibrary.CreateDynamicMaterialInstance` "/Game/Homework/Blueprints/BlackBoard/M_Pixel.M_Pixel"))
      (`KismetArrayLibrary.Array_Add` _materialcollection_4 _returnvalue_3)
      (`MaterialInstanceDynamic.SetVectorParameterValue` (`KismetArrayLibrary.Array_Get` _materialcollection_4 2) "Color" (`KismetMathLibrary.MakeColor` 0.0 1.0 0.0)))
    (:`then_3`
      (bind _returnvalue_4 (`KismetMaterialLibrary.CreateDynamicMaterialInstance` "/Game/Homework/Blueprints/BlackBoard/M_Pixel.M_Pixel"))
      (`KismetArrayLibrary.Array_Add` _materialcollection _returnvalue_4)
      (`MaterialInstanceDynamic.SetVectorParameterValue` (`KismetArrayLibrary.Array_Get` _materialcollection 3) "Color" (`KismetMathLibrary.MakeColor` 0.0 0.0 1.0)))))

(fn `FindRowsAndColumns`
  (`|ExecutionSequence`
    (:`then_0`
      (set `self.columns` (`KismetMathLibrary.FCeil` (/ (`self.width`) (`self.TruePixelSize`)))))
    (:`then_1`
      (set `self.rows` (`KismetMathLibrary.FCeil` (/ (`self.height`) (`self.TruePixelSize`)))))
    (:`then_2`
      (set `self.initPosition` (`self.TopCorner`)))))

(fn `UserConstructionScript`
  (`self.FindRowsAndColumns`)
  (`self.BuildMaterialCollection`)
  (`/Game/Homework/Blueprints/BlackBoard/BPC_GridArray.SetArraySize` (`self.GridArray`) (`self.rows`) (`self.columns`) (- (`KismetArrayLibrary.Array_Length` (`self.materialCollection`)) 1)))