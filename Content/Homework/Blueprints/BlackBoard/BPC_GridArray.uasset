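; BPC_GridArray is a Blueprint component that stores a 2D integer grid in a flat array, sized by Rows and Columns.
; InitArray appends zeros, and GetCell and SetCell address cells through Index, with writes clamped to 0..MaxVal.
; Index holds a row-major formula, but it is left unused.
; ResetArray only prints values because its write is disconnected, and the Grid OnRep prints a debug message.
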(fn `GetCell`
  (params (i :type Integer :default 0) (j :type Integer :default 0))
  (returns (Val :type Integer))
  (return (`KismetArrayLibrary.Array_Get` (`self.grid`) (`self.Index` i j))))

(fn `InitArray`
  (for _ (range 1 (+ (`self.rows`) 1))
    (for _ (range 1 (+ (`self.columns`) 1))
      (`KismetArrayLibrary.Array_Add` (`self.grid`))))
  (`KismetSystemLibrary.PrintString` (`KismetStringLibrary.BuildString_Int` "" "Initialized " (`KismetArrayLibrary.Array_Length` (`self.grid`)) " cells")))

(fn `OnRep_grid`
  (`KismetSystemLibrary.PrintString` "Change dude"))

(fn `ResetArray`
  (for _index (range (`self.rows`))
    (for _index_2 (range (`self.columns`))
      (`KismetSystemLibrary.PrintString` (`KismetStringLibrary.BuildString_Int` "" "Val before:" (`KismetArrayLibrary.Array_Get` (`self.grid`) (`self.Index` _index _index_2)))))))

(fn `SetArraySize`
  (params (r :type Integer :default 0) (c :type Integer :default 0) (max :type Integer :default 0))
  (`|ExecutionSequence`
    (:`then_0`
      (set `self.rows` r))
    (:`then_1`
      (set `self.columns` c))
    (:`then_2`
      (set `self.maxVal` max))))

(fn `SetCell`
  (params (i :type Integer :default 0) (j :type Integer :default 0) (val :type Integer :default 0))
  (`KismetArrayLibrary.Array_Set` (`self.grid`) (`self.Index` i j) (`KismetMathLibrary.Clamp` val 0 (`self.maxVal`))))