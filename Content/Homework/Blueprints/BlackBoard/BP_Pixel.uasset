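; BP_Pixel is a single cell of a blackboard's pixel grid in a homework project.
; It stores its row and column and a parent board reference, all set through setter functions, along with functions for its shape's material and world scale.
; The Draw event passes the cell's indices and a value to the parent's PixelUpdate, leaving the update to the board.
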(event `self.Draw`
  (params (Value :type Integer))
  (bind (_r _c) (`self.GetIndex`))
  (`/Game/Homework/Blueprints/BlackBoard/BP_BlackBoard.PixelUpdate` (`self.parent`) _r _c Value))

(fn `GetIndex`
  (returns (R :type Integer) (C :type Integer))
  (return (`self.Row`) (`self.Column`)))

(fn `SetIndex`
  (params (R :type Integer :default 0) (C :type Integer :default 0))
  (set `self.Row` R)
  (set `self.Column` C))

(fn `SetMaterial`
  (params (mat :type "MaterialInstanceDynamic Object Reference"))
  (`PrimitiveComponent.SetMaterial` (`self.PixelShape`) 0 mat))

(fn `SetParent`
  (params (bb :type "/Game/Homework/Blueprints/BlackBoard/BP_BlackBoard Object Reference"))
  (set `self.parent` bb))

(fn `SetScale`
  (params (s :type "Float (double-precision)" :default 0.0))
  (`SceneComponent.SetWorldScale3D` (`self.PixelShape`) (`KismetMathLibrary.MakeVector` s s s)))

(fn `UserConstructionScript`)