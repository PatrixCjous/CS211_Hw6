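; BP_SessionLeaverM is a trigger actor that makes the local player leave the game session on contact.
; A timeline starts on BeginPlay and animates the Box's world scale uniformly, restarting itself through a custom event each time it finishes.
; When a Character controlled by a local player controller begins overlapping the Box, it calls LeaveGame on the MeetingGameInstance.
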(event `self.ReceiveBeginPlay`
  (bind (_direction _scale) (`Timeline|Anim` :!via `PlayFromStart` :!label _label)
    (:`Update`
      (`SceneComponent.SetWorldScale3D` (`self.Box`) (`KismetMathLibrary.MakeVector` _scale _scale _scale)))
    (:`Finished`
      (`self.LoopDeLoop`))))

(event `LoopDeLoop`
  (goto _label :!via `PlayFromStart`))

(event `self.Box.OnComponentBeginOverlap`
  (params (OtherActor :type "Actor Object Reference") (OtherComp :type "PrimitiveComponent Object Reference") (OtherBodyIndex :type Integer) (bFromSweep :type Boolean) (SweepResult :type "EngineTypes.HitResult Structure (by ref)"))
  (bind _ascharacter (cast `Character` OtherActor))
  (if (`Controller.IsLocalPlayerController` (`Pawn.GetController` _ascharacter))
    (bind _asmeeting_game_instance (cast `/Game/Homework/Blueprints/MeetingGameInstance` (`GameplayStatics.GetGameInstance`)))
    (`/Game/Homework/Blueprints/MeetingGameInstance.LeaveGame` _asmeeting_game_instance)))

(fn `UserConstructionScript`)