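; BP_Message is an in-world message actor showing main, extra and end text that can fade in and out.
; The construction script applies one dynamic material to all three texts, so timelines animate their shared Opacity.
; FadeInOut chains fade-in, Wait, then FadeOut or FadeOutForever, but the Delay inside the Wait event does not pause these functions.
; FadeOutForever disables input and destroys the actor without calling Disappear.
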(event `Wait`
  (params (Time :type "Float (double-precision)"))
  (`KismetSystemLibrary.Delay` Time))

(event `Appear`
  (bind (_direction _opacity) (`Timeline|AlphaIncrease` :!via `PlayFromStart`)
    (:`Update`
      (`MaterialInstanceDynamic.SetScalarParameterValue` (`self.dynMat`) "Opacity" _opacity))))

(event `Disappear`
  (bind (_direction _opacity) (`Timeline|AlphaDecrease` :!via `PlayFromStart`)
    (:`Update`
      (`MaterialInstanceDynamic.SetScalarParameterValue` (`self.dynMat`) "Opacity" _opacity))))

(fn `FadeIn`
  (`self.Appear`)
  (set `self.Shown` true))

(fn `FadeInOut`
  (params (Time :type "Float (double-precision)" :default 0.0) (Destroy :type Boolean))
  (`self.FadeIn`)
  (`self.Wait` (+ Time 5.0))
  (if Destroy
    (`self.FadeOutForever`)
    (else
      (`self.FadeOut`))))

(fn `FadeOut`
  (`self.Disappear`))

(fn `FadeOutForever`
  (`self.DisableInput` null)
  (`self.Wait` 5.0)
  (`self.K2_DestroyActor`))

(fn `SetMessage`
  (bind _endtext (`self.EndText`))
  (bind _extratext (`self.ExtraText`))
  (bind _maintext (`self.MainText`))
  (`|ExecutionSequence`
    (:`then_0`
      (`PrimitiveComponent.SetMaterial` _maintext 0 (`self.dynMat`))
      (`TextRenderComponent.SetText` _maintext (`self.MainTextString`)))
    (:`then_1`
      (`PrimitiveComponent.SetMaterial` _extratext 0 (`self.dynMat`))
      (`TextRenderComponent.SetText` _extratext (`self.ExtraTextString`)))
    (:`then_2`
      (`PrimitiveComponent.SetMaterial` _endtext 0 (`self.dynMat`))
      (`TextRenderComponent.SetText` _endtext (`self.EndTextString`)))))

(fn `UserConstructionScript`
  (bind _returnvalue (`KismetMaterialLibrary.CreateDynamicMaterialInstance` (`self.TextMaterial`)))
  (set `self.dynMat` _returnvalue)
  (`self.SetMessage`))