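; Game instance that handles multiplayer sessions for hosting, joining and leaving a game.
; Hosting creates a four-connection session, optionally on LAN, then opens the game level as a listen server.
; Joining searches for sessions and joins the first result, without using the Combination input that both host and join events receive.
; Leaving destroys the session and opens the lobby level, also with the listen option.
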(event `LeaveGame`
  (`DestroySessionCallbackProxy.DestroySession` (`GameplayStatics.GetPlayerController` 0)
    (:`OnSuccess`
      (`GameplayStatics.OpenLevel` (`self.LobbyLevelString`) true "listen"))))

(event `HostGameEvent`
  (params (Combination :type Integer :default 0))
  (`CreateSessionCallbackProxy.CreateSession` (`GameplayStatics.GetPlayerController` 0) 4 (`self.UseLan?`)
    (:`OnSuccess`
      (`GameplayStatics.OpenLevel` (`self.LevelString`) true "listen"))))

(event `JoinGame`
  (params (Combination :type Integer))
  (bind _results (`FindSessionsCallbackProxy.FindSessions` (`GameplayStatics.GetPlayerController` 0) 4 (`self.UseLan?`))
    (:`OnSuccess`
      (if (not (== (`KismetArrayLibrary.Array_Length` _results) 0))
        (`JoinSessionCallbackProxy.JoinSession` (`GameplayStatics.GetPlayerController` 0) (`KismetArrayLibrary.Array_Get` _results))))))