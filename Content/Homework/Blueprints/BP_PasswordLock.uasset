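; BP_PasswordLock is a four-digit combination lock built from spawned BP_NumberDial actors.
; On BeginPlay it spawns one dial at the world transform of each of its N1–N4 components and stores them as D1–D4.
; GetCombination reads each dial's Number and combines them by place value into a single number, with D1 as the thousands digit.
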(event `self.ReceiveBeginPlay`
  (`|ExecutionSequence`
    (:`then_0`
      (bind _returnvalue (`|SpawnActorFromClass` "/Game/Homework/Blueprints/BP_NumberDial.BP_NumberDial_C" (`SceneComponent.K2_GetComponentToWorld` (`self.N1`)) true))
      (set `self.D1` _returnvalue))
    (:`then_1`
      (bind _returnvalue_2 (`|SpawnActorFromClass` "/Game/Homework/Blueprints/BP_NumberDial.BP_NumberDial_C" (`SceneComponent.K2_GetComponentToWorld` (`self.N2`)) true))
      (set `self.D2` _returnvalue_2))
    (:`then_2`
      (bind _returnvalue_3 (`|SpawnActorFromClass` "/Game/Homework/Blueprints/BP_NumberDial.BP_NumberDial_C" (`SceneComponent.K2_GetComponentToWorld` (`self.N3`)) true))
      (set `self.D3` _returnvalue_3))
    (:`then_3`
      (bind _returnvalue_4 (`|SpawnActorFromClass` "/Game/Homework/Blueprints/BP_NumberDial.BP_NumberDial_C" (`SceneComponent.K2_GetComponentToWorld` (`self.N4`)) true))
      (set `self.D4` _returnvalue_4))))

(fn `GetCombination`
  (returns (Combination :type Integer))
  (return (+ (* (`/Game/Homework/Blueprints/BP_NumberDial.Number` (`self.D1`)) 1000) (* (`/Game/Homework/Blueprints/BP_NumberDial.Number` (`self.D2`)) 100) (* (`/Game/Homework/Blueprints/BP_NumberDial.Number` (`self.D3`)) 10) (`/Game/Homework/Blueprints/BP_NumberDial.Number` (`self.D4`)))))

(fn `UserConstructionScript`)