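; BP_NumberDial is a rotating number dial that steps through digits zero to nine, apparently when a trace hits it.
; Each hit advances Number with wraparound and adds RotationJump to the target rotation, keeping the previous value.
; A RotateSmoothly timeline then lerps the actor's roll between the previous and current rotation while preserving pitch and yaw.
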(event `self.TraceHitActorWithComponent`
  (params (Component :type "PrimitiveComponent Object Reference"))
  (bind (_returnvalue_pitch _returnvalue_yaw) (`KismetMathLibrary.BreakRotator` (`self.K2_GetActorRotation`)))
  (`self.ChangeNumber`)
  (bind (_direction _rotation) (`Timeline|RotateSmoothly` :!via `PlayFromStart`)
    (:`Update`
      (`self.SetActorRotation` (`KismetMathLibrary.MakeRotator` _returnvalue_pitch _returnvalue_yaw (`KismetMathLibrary.Lerp` (`self.PreviousRotation`) (`self.CurrentRotation`) _rotation))))))

(fn `ChangeNumber`
  (set `self.Number` (mod (+ (`self.Number`) 1) 10))
  (set `self.PreviousRotation` (`self.CurrentRotation`))
  (set `self.CurrentRotation` (+ (`self.CurrentRotation`) (`self.RotationJump`))))

(fn `UserConstructionScript`)